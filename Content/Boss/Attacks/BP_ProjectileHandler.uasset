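; BP_ProjectileHandler is a short-lived boss attack actor that launches a series of BP_Projectile actors at a target.
; After a brief delay on BeginPlay, a looping timer acts as a spaced for loop, counting down NProjectiles until it clears itself.
; Each projectile spawns at the handler's location with random pitch and yaw, then receives the handler's Target.
; Tick spins the visible mesh by a fixed, frame-rate-dependent yaw step.
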(event `self.ReceiveBeginPlay`
  (`self.SetLifeSpan` 4.35)
  (`KismetSystemLibrary.Delay` 1.0)
  ;[1 1 1] Timer used as a for loop with 0.7 sec delay b/w each iteration
  (bind _returnvalue (`KismetSystemLibrary.K2_SetTimerDelegate` (delegate `SpawnProjectile`) 0.8 true)))

(event `SpawnProjectile`
  (bind _returnvalue (`|SpawnActorFromClass` "/Game/Boss/Attacks/BP_Projectile.BP_Projectile_C" (`KismetMathLibrary.MakeTransform` (`self.K2_GetActorLocation`) (`KismetMathLibrary.MakeRotator` 0.0 (`KismetMathLibrary.RandomFloatInRange` 0.0 30.0) (`KismetMathLibrary.RandomFloatInRange` -80.0 80.0))) "Undefined" "MultiplyWithRoot" null null))
  (set `/Game/Boss/Attacks/BP_Projectile.Target` (`self.Target`) _returnvalue)
  (bind _result (`/Engine/EditorBlueprintResources/StandardMacros.DecrementInt` (`self.NProjectiles`))
    (:`  `
      ;[1 1 1] For loop end
      (if (== _result 0)
        (`KismetSystemLibrary.K2_ClearAndInvalidateTimerHandle` (stale `self.ReceiveBeginPlay` _returnvalue))))))

(event `self.ReceiveTick`
  (params (DeltaSeconds :type "Float (single-precision)"))
  (bind _staticmesh (`self.StaticMesh`))
  (bind (_returnvalue_roll _returnvalue_pitch _returnvalue_yaw) (`KismetMathLibrary.BreakRotator` (`SceneComponent.K2_GetComponentRotation` _staticmesh)))
  ;[1 1 1] Mesh rotation, the one u see in viewport
  (`SceneComponent.K2_SetWorldRotation` _staticmesh (`KismetMathLibrary.MakeRotator` _returnvalue_roll _returnvalue_pitch (+ _returnvalue_yaw 1.0)) false false))

(fn `UserConstructionScript`)