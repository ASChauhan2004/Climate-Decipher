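; Boss attack actor for a poison cloud hazard that damages its Target for being at or beyond a set distance from the actor, leaving the area inside that radius safe.
; Tick stays off for a short grace period after spawn, and the actor expires on a fixed lifespan.
; A Delay inside Tick throttles the distance check and small damage hit to roughly once per second.
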(event `self.ReceiveBeginPlay`
  (`self.SetActorTickEnabled` false)
  (`self.SetLifeSpan` 48.0)
  (`KismetSystemLibrary.Delay` 3.0)
  (`self.SetActorTickEnabled` true))

(event `self.ReceiveTick`
  (params (DeltaSeconds :type "Float (single-precision)"))
  (bind _target (`self.Target`))
  (`KismetSystemLibrary.Delay` 1.0)
  (if (>= (`self.GetDistanceTo` _target self) 3750.0)
    (`GameplayStatics.ApplyDamage` _target 1.0)))

(fn `UserConstructionScript`)