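; Homing missile projectile for boss attacks, with a limited lifespan.
; It flies without a target briefly, then locks onto the target's capsule with a short burst of extreme homing acceleration to snap its turn before easing to normal homing.
; Overlapping anything destroys it, launching any Character hit along its forward vector.
; Ending play, by impact or timeout, spawns a blast effect and applies radial damage.
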(event `self.ReceiveBeginPlay`
  (bind _projectilemovement (`self.ProjectileMovement`))
  (`self.SetLifeSpan` 9.5)
  ;[1 1 1] The homing part of the homing missle, initally, we dont set any target and it goes in random dir. after some delay we set the target component and increase homing magnitude to jackshit, making it turn rapidly towards u, ofc we need to set it back to some normal value or it will fuck up the player
  (`KismetSystemLibrary.Delay` 0.5)
  (set `ProjectileMovementComponent.HomingTargetComponent` (`Character.CapsuleComponent` (`self.Target`)) _projectilemovement)
  (set `ProjectileMovementComponent.HomingAccelerationMagnitude` 100000.0 _projectilemovement)
  (`KismetSystemLibrary.Delay` 0.1)
  (set `ProjectileMovementComponent.HomingAccelerationMagnitude` 5000.0 _projectilemovement))

(event `self.ReceiveEndPlay`
  (params (EndPlayReason :type "EEndPlayReason Enum" :default "Destroyed"))
  (bind _returnvalue (`self.K2_GetActorLocation`))
  ;[1 1 1] When projectile is about to die, play vfx and add radial damage around it
  (`NiagaraFunctionLibrary.SpawnSystemAtLocation` "/Game/Boss/VFX/NS_ProjectileBlast.NS_ProjectileBlast" _returnvalue)
  (`GameplayStatics.ApplyRadialDamage` :`BaseDamage` 35.0 :`Origin` _returnvalue :`DamageRadius` 200.0 :`DamageCauser` null :`InstigatedByController` null))

(event `self.Sphere.OnComponentBeginOverlap`
  (params (OverlappedComponent :type "PrimitiveComponent Object Reference") (OtherActor :type "Actor Object Reference") (OtherComp :type "PrimitiveComponent Object Reference") (OtherBodyIndex :type Integer) (bFromSweep :type Boolean) (SweepResult :type "HitResult Structure (by ref)"))
  ;[1 1 1] If overlapped with some object, destroy the actor. If its a character then launch the character
  (bind _ascharacter (cast `Character` OtherActor)
    (:`then`
      (`Character.LaunchCharacter` _ascharacter (* (`self.GetActorForwardVector`) 2000.0) false false))
    (:`CastFailed`
      _))
  (`self.K2_DestroyActor`))

(fn `UserConstructionScript`)